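; Forcefield actor that reacts to arrow hits on its sphere and breaks after repeated impacts.
; Each Arrowactor hit is stored, spawns debris, and drives a dynamic material ripple by setting the impact position and animating its radius with a timeline.
; A damage counter feeds the material's amount parameter and rises per hit; at its threshold the forcefield destroys itself and the stored arrows.
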(event OnComponentHit(Sphere)
  (params (HitComponent :type Primitive%20Component%20Object%20Reference) (OtherActor :type Actor%20Object%20Reference) (OtherComp :type Primitive%20Component%20Object%20Reference) (NormalImpulse :type Vector :default "0, 0, 0") (Hit :type Hit%20Result%20Structure%20%28by%20ref%29))
  (bind _asarrowactor (Utilities|Casting|CastToArrowactor OtherActor))
  (if (== OtherActor _asarrowactor)
    (Utilities|Array|Add (Variables|Default|GetNewVar_1) OtherActor))
  (Utilities|FlowControl|Sequence
    (:then_0
      (bind _returnvalue (Rendering|Material|CreateDynamicMaterialInstance (Variables|Default|GetSphere1) 0 0 :!class /Script/Engine.PrimitiveComponent))
      (Effects|SpawnEmitteratLocation "/Game/pratice/wonseok/Material/debri.debri" (.impactpoint Hit) (Math|Rotator|MakeRotfromX (.impactnormal Hit)))
      (Rendering|Material|SetVectorParameterValue _returnvalue "Pos" (Math|Conversions|ToLinearColor(Vector) (.impactpoint Hit)) :!class /Script/Engine.MaterialInstanceDynamic)
      (bind _새_트랙_0 (Timeline|타임라인_0 PlayFromStart)
        (:Update
          (Rendering|Material|SetScalarParameterValue _returnvalue "radius" (* _새_트랙_0 2e+02) :!class /Script/Engine.MaterialInstanceDynamic))))
    (:then_1
      (bind _returnvalue_2 (Rendering|Material|CreateDynamicMaterialInstance (Variables|Default|GetSphere1) 0 0 :!class /Script/Engine.PrimitiveComponent))
      (Rendering|Material|SetScalarParameterValue _returnvalue_2 "amount" (Variables|Default|GetNewVar_0) :!class /Script/Engine.MaterialInstanceDynamic)
      (Variables|Default|SetNewVar_0 (+ (Variables|Default|GetNewVar_0) 0.2)))
    (:then_2
      (if (>= (Variables|Default|GetNewVar_0) 1.0)
        (Actor|DestroyActor)
        (for _array_element (Variables|Default|GetNewVar_1)
          (Actor|DestroyActor _array_element))))))

(event EventBeginPlay)

(event Collision|EventActorBeginOverlap
  (params (OtherActor :type Actor%20Object%20Reference)))

(event EventTick
  (params (DeltaSeconds :type Float%20%28single-precision%29)))

(fn ConstructionScript)