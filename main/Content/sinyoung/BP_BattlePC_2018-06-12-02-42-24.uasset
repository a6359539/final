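; Battle player controller that runs the multiplayer lobby and the handoff into a Blue versus Red match.
; It shows the ready widget, spawns a switchable lobby character (Kwangsword or Shinbibow), relays chat and manages team slots, ready checks and room master.
; Changes loop through all controllers to refresh slots from the GameMode's player list, with a Servecheck macro splitting server from owning client.
; A countdown ends by spawning and possessing the team character.
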(event Custom|tryready
  (if (!= (Variables|Default|GetTeam) 0)
    (if (Variables|Default|Getb_ready)
      (Variables|Default|Setb_ready false)
      (else
        (Variables|Default|Setb_ready true)))
    (CallFunction|Multicast)
    (bind _asbp_battle_gm (Utilities|Casting|CastToBP_BattleGM (Game|GetGameMode)))
    (Default|Checkallready _asbp_battle_gm)))

(event Custom|ReadyWidget
  (bind _asmy_game_instance (Utilities|Casting|CastToMyGameInstance (Game|GetGameInstance)))
  (Variables|Default|SetPlayerName (Variables|/Game/Battle/MyGameInstance.MyGameInstance_C|GetMyPlayerName _asmy_game_instance))
  (CallFunction|SetPlayerName (Variables|/Game/Battle/MyGameInstance.MyGameInstance_C|GetMyPlayerName _asmy_game_instance)))

(event Custom|respawnchar
  (bind _returnvalue (Game|GetGameMode))
  (bind _asbp_battle_gm (Utilities|Casting|CastToBP_BattleGM _returnvalue))
  (bind _lobbystart (Variables|/Game/Battle/BP_BattleGM_2018-03-20-20-26-08.BP_BattleGM_C|Getlobbystart _asbp_battle_gm))
  (switch int (Variables|Default|Getchartype)
    (:0
      (bind _returnvalue_2 (Game|SpawnActorfromClass "/Game/sinyoung/shinbi/kwangsword.kwangsword_C" _lobbystart "Undefined" 0 true 0))
      (bind _output_get (Variables|Default|Setlobbykwangchar _returnvalue_2))
      (Pawn|Possess _output_get))
    (:1
      (bind _returnvalue_3 (Game|SpawnActorfromClass "/Game/sinyoung/shinbi/shinbibow.shinbibow_C" _lobbystart "Undefined" 0 true 0))
      (bind _output_get_2 (Variables|Default|Setlobbyshinbichar _returnvalue_3))
      (Pawn|Possess _output_get_2))))

(event Custom|startvisivle
  (Widget|SetVisibility (Variables|/Game/Battle/Widget_Ready.Widget_Ready_C|Getstartt (Variables|Default|GetReadyW)) "Visible"))

(event Custom|defaultfreeteam
  (if (not (Variables|Default|Getb_ready))
    (Variables|Default|SetTeam 0)
    (if (Utilities|Enum|Equal(Enum) (Utilities|Text|ToText(String) (Variables|free|Getfree1)) (Class|KismetTextLibrary|GetEmptyText))
      (Variables|Default|SetTeamindex 1)
      (CallFunction|Multicast :!label _label)
      (elif (Utilities|Enum|Equal(Enum) (Utilities|Text|ToText(String) (Variables|free|Getfree2)) (Class|KismetTextLibrary|GetEmptyText))
        (Variables|Default|SetTeamindex 2)
        (goto _label)
        (elif (Utilities|Enum|Equal(Enum) (Utilities|Text|ToText(String) (Variables|free|Getfree3)) (Class|KismetTextLibrary|GetEmptyText))
          (Variables|Default|SetTeamindex 3)
          (goto _label)
          (elif (Utilities|Enum|Equal(Enum) (Utilities|Text|ToText(String) (Variables|free|Getfree4)) (Class|KismetTextLibrary|GetEmptyText))
            (Variables|Default|SetTeamindex 4)
            (goto _label)
            (elif (Utilities|Enum|Equal(Enum) (Utilities|Text|ToText(String) (Variables|free|Getfree5)) (Class|KismetTextLibrary|GetEmptyText))
              (Variables|Default|SetTeamindex 5)
              (goto _label)
              (elif (Utilities|Enum|Equal(Enum) (Utilities|Text|ToText(String) (Variables|free|Getfree6)) (Class|KismetTextLibrary|GetEmptyText))
                (Variables|Default|SetTeamindex 6)
                (goto _label)
                (elif (Utilities|Enum|Equal(Enum) (Utilities|Text|ToText(String) (Variables|free|Getfree7)) (Class|KismetTextLibrary|GetEmptyText))
                  (Variables|Default|SetTeamindex 7)
                  (goto _label)
                  (elif (Utilities|Enum|Equal(Enum) (Utilities|Text|ToText(String) (Variables|free|Getfree8)) (Class|KismetTextLibrary|GetEmptyText))
                    (Variables|Default|SetTeamindex 8)
                    (goto _label)))))))))))

(event Custom|setredteam
  (Utilities|Servecheck
    (:server
      (if (not (Variables|Default|Getb_ready))
        (if (!= (Variables|Default|GetTeam) 2)
          (Variables|Default|SetTeam 2)
          (if (Utilities|Enum|Equal(Enum) (Utilities|Text|ToText(String) (Variables|Redteam|Getred1)) (Utilities|Text|FormatText "빈 슬롯"))
            (Variables|Default|SetTeamindex 1)
            (CallFunction|Multicast :!label _label)
            (elif (Utilities|Enum|Equal(Enum) (Utilities|Text|ToText(String) (Variables|Redteam|Getred2)) (Utilities|Text|FormatText "빈 슬롯"))
              (Variables|Default|SetTeamindex 2)
              (goto _label)
              (elif (Utilities|Enum|Equal(Enum) (Utilities|Text|ToText(String) (Variables|Redteam|Getred3)) (Utilities|Text|FormatText "빈 슬롯"))
                (Variables|Default|SetTeamindex 3)
                (goto _label)
                (elif (Utilities|Enum|Equal(Enum) (Utilities|Text|ToText(String) (Variables|Redteam|Getred4)) (Utilities|Text|FormatText "빈 슬롯"))
                  (Variables|Default|SetTeamindex 4)
                  (goto _label)
                  (elif (Utilities|Enum|Equal(Enum) (Utilities|Text|ToText(String) (Variables|Redteam|Getred5)) (Utilities|Text|FormatText "빈 슬롯"))
                    (Variables|Default|SetTeamindex 5)
                    (goto _label)))))))))))

(event Custom|starthidden
  (Widget|SetVisibility (Variables|/Game/Battle/Widget_Ready.Widget_Ready_C|Getstartt (Variables|Default|GetReadyW)) "Hidden"))

(event Custom|readyhidden
  (params (team :type Integer) (index :type Integer))
  (bind _readyw (Variables|Default|GetReadyW))
  (switch int team
    (:1
      (switch int index
        (:1
          (Widget|SetVisibility (Variables|/Game/Battle/Widget_Ready.Widget_Ready_C|Getbluereadycheck1 _readyw) "Hidden"))
        (:2
          (Widget|SetVisibility (Variables|/Game/Battle/Widget_Ready.Widget_Ready_C|Getbluereadycheck2 _readyw) "Hidden"))
        (:3
          (Widget|SetVisibility (Variables|/Game/Battle/Widget_Ready.Widget_Ready_C|Getbluereadycheck3 _readyw) "Hidden"))
        (:4
          (Widget|SetVisibility (Variables|/Game/Battle/Widget_Ready.Widget_Ready_C|Getbluereadycheck4 _readyw) "Hidden"))))
    (:2
      (switch int index
        (:1
          (Widget|SetVisibility (Variables|/Game/Battle/Widget_Ready.Widget_Ready_C|Getredreadycheck1 _readyw) "Hidden"))
        (:2
          (Widget|SetVisibility (Variables|/Game/Battle/Widget_Ready.Widget_Ready_C|Getredreadycheck2 _readyw) "Hidden"))
        (:3
          (Widget|SetVisibility (Variables|/Game/Battle/Widget_Ready.Widget_Ready_C|Getredreadycheck3 _readyw) "Hidden"))
        (:4
          (Widget|SetVisibility (Variables|/Game/Battle/Widget_Ready.Widget_Ready_C|Getredreadycheck4 _readyw) "Hidden"))
        (:5
          (Widget|SetVisibility (Variables|/Game/Battle/Widget_Ready.Widget_Ready_C|Getredreadycheck5 _readyw) "Hidden"))))))

(event Custom|startgame
  (bind _asbp_battle_gm (Utilities|Casting|CastToBP_BattleGM (Game|GetGameMode)))
  (Variables|/Game/Battle/BP_BattleGM_2018-03-20-20-26-08.BP_BattleGM_C|SetPlayingState _asbp_battle_gm "NewEnumerator0"))

(event Custom|set%20realchar
  (bind _returnvalue (Game|GetGameMode))
  (bind _chartype (Variables|Default|Getchartype))
  (bind _asbp_battle_gm (Utilities|Casting|CastToBP_BattleGM _returnvalue))
  (bind _redteamspawn (Variables|/Game/Battle/BP_BattleGM_2018-03-20-20-26-08.BP_BattleGM_C|GetRedteamspawn _asbp_battle_gm))
  (bind _blueteamspawn (Variables|/Game/Battle/BP_BattleGM_2018-03-20-20-26-08.BP_BattleGM_C|GetBlueteamspawn _asbp_battle_gm))
  (Pawn|UnPossess)
  (Actor|DestroyActor (Variables|Default|Getlobbykwangchar))
  (if (== (Variables|Default|GetTeam) 1)
    (switch int _chartype
      (:0
        (bind _returnvalue_2 (Game|SpawnActorfromClass "/Game/sinyoung/shinbi/kwangsword.kwangsword_C" _blueteamspawn "Undefined" self false 0))
        (Variables|Default|Setmy%20char _returnvalue_2)
        (Pawn|Possess _returnvalue_2))
      (:1
        (bind _returnvalue_3 (Game|SpawnActorfromClass "/Game/sinyoung/shinbi/shinbibow.shinbibow_C" _blueteamspawn "Undefined" self false 0))
        (Variables|Default|Setmy%20char _returnvalue_3)
        (Pawn|Possess _returnvalue_3)))
    (else
      (switch int _chartype
        (:0
          (bind _returnvalue_4 (Game|SpawnActorfromClass "/Game/sinyoung/shinbi/kwangsword.kwangsword_C" _redteamspawn "Undefined" self false 0))
          (Variables|Default|Setmy%20char _returnvalue_4)
          (Pawn|Possess _returnvalue_4))
        (:1
          (bind _returnvalue_5 (Game|SpawnActorfromClass "/Game/sinyoung/shinbi/shinbibow.shinbibow_C" _redteamspawn "Undefined" self false 0))
          (Variables|Default|Setmy%20char _returnvalue_5)
          (Pawn|Possess _returnvalue_5))))))

(event Custom|readyvisible
  (params (team :type Integer) (index :type Integer))
  (bind _readyw (Variables|Default|GetReadyW))
  (switch int team
    (:1
      (switch int index
        (:1
          (Widget|SetVisibility (Variables|/Game/Battle/Widget_Ready.Widget_Ready_C|Getbluereadycheck1 _readyw) "Visible"))
        (:2
          (Widget|SetVisibility (Variables|/Game/Battle/Widget_Ready.Widget_Ready_C|Getbluereadycheck2 _readyw) "Visible"))
        (:3
          (Widget|SetVisibility (Variables|/Game/Battle/Widget_Ready.Widget_Ready_C|Getbluereadycheck3 _readyw) "Visible"))
        (:4
          (Widget|SetVisibility (Variables|/Game/Battle/Widget_Ready.Widget_Ready_C|Getbluereadycheck4 _readyw) "Visible"))))
    (:2
      (switch int index
        (:1
          (Widget|SetVisibility (Variables|/Game/Battle/Widget_Ready.Widget_Ready_C|Getredreadycheck1 _readyw) "Visible"))
        (:2
          (Widget|SetVisibility (Variables|/Game/Battle/Widget_Ready.Widget_Ready_C|Getredreadycheck2 _readyw) "Visible"))
        (:3
          (Widget|SetVisibility (Variables|/Game/Battle/Widget_Ready.Widget_Ready_C|Getredreadycheck3 _readyw) "Visible"))
        (:4
          (Widget|SetVisibility (Variables|/Game/Battle/Widget_Ready.Widget_Ready_C|Getredreadycheck4 _readyw) "Visible"))
        (:5
          (Widget|SetVisibility (Variables|/Game/Battle/Widget_Ready.Widget_Ready_C|Getredreadycheck5 _readyw) "Visible"))))))

(event Custom|playwaittime
  (params (waittime :type Integer))
  (Utilities|FlowControl|Sequence
    (:then_0
      (Utilities|FlowControl|DoOnce false
        (:Completed
          (Widget|RemovefromParent (Variables|Default|GetReadyW))
          (Variables|Default|SetbShowMouseCursor false)
          (Variables|Default|Setlobby? false))))
    (:then_1
      (Utilities|FlowControl|DoOnce false
        (:Completed
          (bind _returnvalue (UserInterface|CreateWidget "/Game/Battle/startcountwidget.startcountwidget_C" self))
          (bind _output_get (Variables|Default|Setcountwidget _returnvalue))
          (UserInterface|Viewport|AddtoViewport _output_get 0))))
    (:then_2
      (Variables|/Game/Battle/startcountwidget.startcountwidget_C|Settext (Variables|Default|Getcountwidget) (Utilities|Text|FormatText "{t}초 후 게임이 시작됩니다. " waittime)))
    (:then_3
      (if (== waittime 1)
        (CallFunction|SetRealchar)
        (Utilities|FlowControl|Delay 1.0)
        (Widget|SetVisibility (Variables|Default|Getcountwidget) "Hidden")))))

(event Custom|SetPlayerName
  (params (PlayerName :type String))
  (Class|GameModeBase|ChangeName (Game|GetGameMode) self PlayerName false)
  (Variables|Default|SetPlayerName PlayerName))

(event Custom|setblueteam
  (Utilities|Servecheck
    (:server
      (if (not (Variables|Default|Getb_ready))
        (if (!= (Variables|Default|GetTeam) 1)
          (Variables|Default|SetTeam 1)
          (if (Utilities|Enum|Equal(Enum) (Utilities|Text|ToText(String) (Variables|blueteam|Getblue1)) (Utilities|Text|FormatText "빈 슬롯"))
            (Variables|Default|SetTeamindex 1)
            (bind _asbp_battle_gm (Utilities|Casting|CastToBP_BattleGM (Game|GetGameMode)))
            (Variables|/Game/Battle/BP_BattleGM_2018-03-20-20-26-08.BP_BattleGM_C|Setroommaster _asbp_battle_gm self)
            (CallFunction|Multicast :!label _label)
            (elif (Utilities|Enum|Equal(Enum) (Utilities|Text|ToText(String) (Variables|blueteam|Getblue2)) (Utilities|Text|FormatText "빈 슬롯"))
              (Variables|Default|SetTeamindex 2)
              (goto _label)
              (elif (Utilities|Enum|Equal(Enum) (Utilities|Text|ToText(String) (Variables|blueteam|Getblue3)) (Utilities|Text|FormatText "빈 슬롯"))
                (Variables|Default|SetTeamindex 3)
                (goto _label)
                (elif (Utilities|Enum|Equal(Enum) (Utilities|Text|ToText(String) (Variables|blueteam|Getblue4)) (Utilities|Text|FormatText "빈 슬롯"))
                  (Variables|Default|SetTeamindex 4)
                  (goto _label)
                  (elif (Utilities|Enum|Equal(Enum) (Utilities|Text|ToText(String) (Variables|blueteam|Getblue5)) (Utilities|Text|FormatText "빈 슬롯"))
                    (Variables|Default|SetTeamindex 5)
                    (goto _label)))))))))))

(event Custom|clearevent
  (Variables|blueteam|Setblue1 "빈 슬롯")
  (Variables|blueteam|Setblue2 "빈 슬롯")
  (Variables|blueteam|Setblue3 "빈 슬롯")
  (Variables|blueteam|Setblue4 "빈 슬롯")
  (Variables|blueteam|Setblue5 "빈 슬롯")
  (Variables|Redteam|Setred1 "빈 슬롯")
  (Variables|Redteam|Setred2 "빈 슬롯")
  (Variables|Redteam|Setred3 "빈 슬롯")
  (Variables|Redteam|Setred4 "빈 슬롯")
  (Variables|Redteam|Setred5 "빈 슬롯")
  (Variables|free|Setfree8 "")
  (Variables|free|Setfree7 "")
  (Variables|free|Setfree6 "")
  (Variables|free|Setfree5 "")
  (Variables|free|Setfree4 "")
  (Variables|free|Setfree3 "")
  (Variables|free|Setfree2 "")
  (Variables|free|Setfree1 ""))

(event Custom|multi
  (Utilities|Servecheck
    (:my
      (CallFunction|Update))))

(event Custom|lobbyspawn
  (Variables|Default|Setchartype 0)
  (bind _returnvalue (Game|SpawnActorfromClass "/Game/sinyoung/shinbi/kwangsword.kwangsword_C" (Variables|/Game/Battle/BP_BattleGM_2018-03-20-20-26-08.BP_BattleGM_C|Getlobbystart (.AsBP%20Battle%20GM (Utilities|Casting|CastToBP_BattleGM (Game|GetGameMode)))) "Undefined" 0 true 0))
  (bind _output_get (Variables|Default|Setlobbykwangchar _returnvalue))
  (Pawn|Possess _output_get))

(event Custom|update
  (Utilities|Servecheck
    (:server
      (CallFunction|Clearevent)
      (bind _asbp_battle_gm (Utilities|Casting|CastToBP_BattleGM (Game|GetGameMode)))
      (for _array_element (Variables|/Game/Battle/BP_BattleGM_2018-03-20-20-26-08.BP_BattleGM_C|GetAlivePCs _asbp_battle_gm)
        (if (Variables|BP_BattlePC_C|Getb_ready _array_element)
          (CallFunction|Readyvisible (Variables|BP_BattlePC_C|GetTeam _array_element) (Variables|BP_BattlePC_C|GetTeamindex _array_element))
          (else
            (CallFunction|Readyhidden (Variables|BP_BattlePC_C|GetTeam _array_element) (Variables|BP_BattlePC_C|GetTeamindex _array_element))))
        (switch int (Variables|BP_BattlePC_C|GetTeam _array_element)
          (:0
            (switch int (Variables|BP_BattlePC_C|GetTeamindex _array_element)
              (:1
                (Variables|free|Setfree1 (Variables|BP_BattlePC_C|GetPlayerName _array_element)))
              (:2
                (Variables|free|Setfree2 (Variables|BP_BattlePC_C|GetPlayerName _array_element)))
              (:3
                (Variables|free|Setfree3 (Variables|BP_BattlePC_C|GetPlayerName _array_element)))
              (:4
                (Variables|free|Setfree4 (Variables|BP_BattlePC_C|GetPlayerName _array_element)))
              (:5
                (Variables|free|Setfree5 (Variables|BP_BattlePC_C|GetPlayerName _array_element)))
              (:6
                (Variables|free|Setfree6 (Variables|BP_BattlePC_C|GetPlayerName _array_element)))
              (:7
                (Variables|free|Setfree7 (Variables|BP_BattlePC_C|GetPlayerName _array_element)))))
          (:1
            (switch int (Variables|BP_BattlePC_C|GetTeamindex _array_element)
              (:1
                (Variables|blueteam|Setblue1 (Variables|BP_BattlePC_C|GetPlayerName _array_element)))
              (:2
                (Variables|blueteam|Setblue2 (Variables|BP_BattlePC_C|GetPlayerName _array_element)))
              (:3
                (Variables|blueteam|Setblue3 (Variables|BP_BattlePC_C|GetPlayerName _array_element)))
              (:4
                (Variables|blueteam|Setblue4 (Variables|BP_BattlePC_C|GetPlayerName _array_element)))
              (:5
                (Variables|blueteam|Setblue5 (Variables|BP_BattlePC_C|GetPlayerName _array_element)))))
          (:2
            (switch int (Variables|BP_BattlePC_C|GetTeamindex _array_element)
              (:1
                (Variables|Redteam|Setred1 (Variables|BP_BattlePC_C|GetPlayerName _array_element)))
              (:2
                (Variables|Redteam|Setred2 (Variables|BP_BattlePC_C|GetPlayerName _array_element)))
              (:3
                (Variables|Redteam|Setred3 (Variables|BP_BattlePC_C|GetPlayerName _array_element)))
              (:4
                (Variables|Redteam|Setred4 (Variables|BP_BattlePC_C|GetPlayerName _array_element)))
              (:5
                (Variables|Redteam|Setred5 (Variables|BP_BattlePC_C|GetPlayerName _array_element))))))))))

(event Custom|sendchatmessage
  (params (message :type Text) (type :type Integer))
  (bind _playername (Variables|Default|GetPlayerName))
  (bind _returnvalue (Utilities|Text|ToText(String) _playername))
  (bind _returnvalue_2 (Class|GameModeBase|GetNumPlayers (Game|GetGameMode)))
  (for _index (range 0 (- _returnvalue_2 1))
    (bind _asbp_battle_pc (Utilities|Casting|CastToBP_BattlePC (Game|GetPlayerController _index)))
    (switch int type
      (:0
        (CallFunction|Addchatmessage _asbp_battle_pc (Utilities|Text|FormatText "{name}님이 방에 들어오셨습니다.!" _returnvalue) type))
      (:1
        (CallFunction|Addchatmessage _asbp_battle_pc (Utilities|Text|FormatText "{name} : {message}" _returnvalue message) type)))))

(event Custom|PCmaintimer
  (bind _askwangsword (Utilities|Casting|CastTokwangsword (Variables|Default|Getmy%20char)))
  (Default|Maintimer _askwangsword))

(event Custom|charchange
  (params (char :type Integer))
  (if (!= char (Variables|Default|Getchartype))
    (Variables|Default|Setchartype char)
    (Pawn|UnPossess)
    (Actor|DestroyActor (Variables|Default|Getlobbykwangchar))
    (Actor|DestroyActor (Variables|Default|Getlobbyshinbichar))
    (CallFunction|Respawnchar)))

(event Custom|addchatmessage
  (params (message :type Text) (type :type Integer))
  (Default|Addchatmessage (Variables|Default|GetReadyW) message type))

(event Custom|multicast
  (Utilities|Servecheck
    (:server
      (bind _returnvalue (Class|GameModeBase|GetNumPlayers (Game|GetGameMode)))
      (for _index (range 0 (- _returnvalue 1))
        (bind _asbp_battle_pc (Utilities|Casting|CastToBP_BattlePC (Game|GetPlayerController _index)))
        (CallFunction|Multi _asbp_battle_pc)))))

(event EventBeginPlay
  (Utilities|Servecheck
    (:my
      (CallFunction|ReadyWidget)
      (bind _returnvalue (UserInterface|CreateWidget "/Game/Battle/Widget_Ready.Widget_Ready_C" self self))
      (Variables|Default|SetReadyW _returnvalue)
      (UserInterface|Viewport|AddtoViewport _returnvalue 0)
      (CallFunction|Lobbyspawn)
      (Variables|Default|SetbShowMouseCursor true)
      (CallFunction|Update)
      (CallFunction|Defaultfreeteam)
      (CallFunction|Sendchatmessage))))

(event EventTick
  (params (DeltaSeconds :type Float%20%28single-precision%29)))

(event Input|KeyboardEvents|Tab
  (params (Key :type Key%20Structure))
  (:Pressed
    (if (Variables|Default|Getlobby?)
      (Utilities|FlowControl|FlipFlop
        (:A
          (Widget|RemovefromParent (Variables|Default|GetReadyW))
          (Variables|Default|SetbShowMouseCursor false)
          (Input|SetInputModeGameOnly self))
        (:B
          (UserInterface|Viewport|AddtoViewport (Variables|Default|GetReadyW) 0)
          (Variables|Default|SetbShowMouseCursor true)
          (Input|SetInputModeGameandUI self 0 "DoNotLock" true))))))

(fn ConstructionScript)