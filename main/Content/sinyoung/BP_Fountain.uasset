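; Team-owned fountain actor that offers relic (sungmul) looting interactions to kwangsword and shinbibow characters, with point lights tinted blue or green for two of its Types.
; Entering the box calls Rootin in mode 2 for enemies while Active, or mode 1 for teammates carrying a matching-type relic while inactive.
; Overlapping actors are tracked in an array, so Rootout runs on exit or for all of them through removewidget.
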(event OnComponentBeginOverlap(Box)
  (params (OverlappedComponent :type Primitive%20Component%20Object%20Reference) (OtherActor :type Actor%20Object%20Reference) (OtherComp :type Primitive%20Component%20Object%20Reference) (OtherBodyIndex :type Integer) (bFromSweep :type Boolean) (SweepResult :type Hit%20Result%20Structure%20%28by%20ref%29))
  (Utilities|Array|Add (Variables|Default|Getobject) OtherActor)
  (bind _askwangsword (Utilities|Casting|CastTokwangsword OtherActor)
    (:then
      (if (Variables|Default|Getactive?)
        (if (!= (Variables|/Game/sinyoung/shinbi/kwangsword.kwangsword_C|Getteam _askwangsword) (Variables|Default|Getteam))
          (Variables|/Game/sinyoung/shinbi/kwangsword.kwangsword_C|Setfinalsungmulactor _askwangsword self)
          (Variables|/Game/sinyoung/shinbi/kwangsword.kwangsword_C|Setroottype _askwangsword (Variables|Default|Gettype))
          (Default|Rootin _askwangsword 2))
        (elif (== (Variables|Default|Getteam) (Variables|/Game/sinyoung/shinbi/kwangsword.kwangsword_C|Getteam _askwangsword))
          (if (Variables|/Game/sinyoung/shinbi/kwangsword.kwangsword_C|Gethavesungmul _askwangsword)
            (if (== (Variables|Default|Gettype) (Variables|/Game/sinyoung/shinbi/kwangsword.kwangsword_C|Getroottype _askwangsword))
              (Variables|/Game/sinyoung/shinbi/kwangsword.kwangsword_C|Setfinalsungmulactor _askwangsword self)
              (Default|Rootin _askwangsword 1))))))
    (:CastFailed
      (bind _asshinbibow (Utilities|Casting|CastToshinbibow OtherActor))
      (if (Variables|Default|Getactive?)
        (if (!= (Variables|/Game/sinyoung/shinbi/shinbibow.shinbibow_C|Getteam _asshinbibow) (Variables|Default|Getteam))
          (Variables|/Game/sinyoung/shinbi/shinbibow.shinbibow_C|Setfinalsungmulactor _asshinbibow self)
          (Variables|/Game/sinyoung/shinbi/shinbibow.shinbibow_C|Setroottype _asshinbibow (Variables|Default|Gettype))
          (Default|Rootin _asshinbibow 2))
        (elif (== (Variables|Default|Getteam) (Variables|/Game/sinyoung/shinbi/shinbibow.shinbibow_C|Getteam _asshinbibow))
          (if (Variables|/Game/sinyoung/shinbi/shinbibow.shinbibow_C|Gethavesungmul _asshinbibow)
            (if (== (Variables|Default|Gettype) (Variables|/Game/sinyoung/shinbi/shinbibow.shinbibow_C|Getroottype _asshinbibow))
              (Variables|/Game/sinyoung/shinbi/shinbibow.shinbibow_C|Setfinalsungmulactor _asshinbibow self)
              (Default|Rootin _asshinbibow 1))))))))

(event OnComponentEndOverlap(Box)
  (params (OverlappedComponent :type Primitive%20Component%20Object%20Reference) (OtherActor :type Actor%20Object%20Reference) (OtherComp :type Primitive%20Component%20Object%20Reference) (OtherBodyIndex :type Integer))
  (Utilities|Array|RemoveItem (Variables|Default|Getobject) OtherActor)
  (bind _askwangsword (Utilities|Casting|CastTokwangsword OtherActor)
    (:then
      (Default|Rootout _askwangsword))
    (:CastFailed
      (bind _asshinbibow (Utilities|Casting|CastToshinbibow OtherActor))
      (Default|Rootout _asshinbibow))))

(event Custom|removewidget
  (for _array_element (Variables|Default|Getobject)
    (bind _askwangsword (Utilities|Casting|CastTokwangsword _array_element)
      (:then
        (Default|Rootout _askwangsword))
      (:CastFailed
        (bind _asshinbibow (Utilities|Casting|CastToshinbibow _array_element))
        (Default|Rootout _asshinbibow)))))

(event EventBeginPlay
  (switch int (Variables|Default|Gettype)
    (:0
      (Rendering|Components|Light|SetLightColor (Variables|Default|GetPointLight) "(R=0.070432,G=0.056845,B=0.979167,A=1.000000)" true)
      (Rendering|Components|Light|SetLightColor (Variables|Default|GetPointLight1) "(R=0.070432,G=0.056845,B=0.979167,A=1.000000)" true)
      (Rendering|Components|Light|SetLightColor (Variables|Default|GetPointLight2) "(R=0.070432,G=0.056845,B=0.979167,A=1.000000)" true)
      (Rendering|Components|Light|SetLightColor (Variables|Default|GetPointLight3) "(R=0.070432,G=0.056845,B=0.979167,A=1.000000)" true))
    (:2
      (Rendering|Components|Light|SetLightColor (Variables|Default|GetPointLight) "(R=0.032795,G=0.979167,B=0.039645,A=1.000000)" true)
      (Rendering|Components|Light|SetLightColor (Variables|Default|GetPointLight1) "(R=0.105276,G=0.979167,B=0.084558,A=1.000000)" true)
      (Rendering|Components|Light|SetLightColor (Variables|Default|GetPointLight2) "(R=0.094637,G=0.979167,B=0.000000,A=1.000000)" true)
      (Rendering|Components|Light|SetLightColor (Variables|Default|GetPointLight3) "(R=0.031038,G=0.979167,B=0.192222,A=1.000000)" true))))

(event Collision|EventActorBeginOverlap
  (params (OtherActor :type Actor%20Object%20Reference)))

(fn ConstructionScript)