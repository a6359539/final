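; Battle game mode that tracks player controllers, runs the start countdown and match clock, and spawns "sungmul" actors.
; A one-second timer drives the Waiting and Battle states, pushing time to controllers and their sword or bow characters.
; Entering Battle schedules three staggered spawns, each rerolling across frames for an unused type, picking a random spawn point and notifying all players.
; It also toggles the room master's start control on all-ready and broadcasts messages.
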(event Custom|MainTimer
  (switch Utilities|FlowControl|Switch|SwitchonEPlayingState (Variables|Default|GetPlayingState)
    (:NewEnumerator0
      (if (> (Variables|Default|Getstartwaittiome) 0)
        (for _array_element (Variables|Default|GetAlivePCs)
          (Default|Playwaittime _array_element (Variables|Default|Getstartwaittiome)))
        (bind _result (Math|Integer|DecrementInt (Variables|Default|Getstartwaittiome))
          (:%20%20
            (Variables|Default|Setstartwaittiome _result)))
        (else
          (Variables|Default|Setstartwaittiome 5)
          (Variables|Default|SetPlayingState "NewEnumerator1")
          (Utilities|Time|SetTimerbyEvent (delegate Custom|se1) 5.0)
          (Utilities|Time|SetTimerbyEvent (delegate Custom|se2) 1e+01)
          (Utilities|Time|SetTimerbyEvent (delegate Custom|se3) 15.0))))
    (:NewEnumerator1
      (bind _result_2 (Math|Float|IncrementFloat (Variables|Default|GetMainTime))
        (:%20%20
          (Variables|Default|SetMainTime _result_2)
          (for _array_element_2 (Variables|Default|GetAlivePCs)
            (Default|PCmaintimer _array_element_2)
            (switch int (Variables|/Game/Battle/BP_BattlePC.BP_BattlePC_C|Getchartype _array_element_2)
              (:0
                (Default|MaintimerSet (.AsKwangsword (Utilities|Casting|CastTokwangsword (Variables|/Game/Battle/BP_BattlePC.BP_BattlePC_C|Getmy%20char _array_element_2))) (Variables|Default|GetMainTime)))
              (:1
                (Default|MaintimerSet (.AsShinbibow (Utilities|Casting|CastToshinbibow (Variables|/Game/Battle/BP_BattlePC.BP_BattlePC_C|Getmy%20char _array_element_2))) (Variables|Default|GetMainTime))))))))))

(event Custom|checkallready
  (bind _roommaster (Variables|Default|Getroommaster))
  (Variables|Default|Setplayernum 0)
  (for _array_element (Variables|Default|GetAlivePCs)
    (if (Variables|/Game/Battle/BP_BattlePC.BP_BattlePC_C|Getb_ready _array_element)
      (bind _result (Math|Integer|IncrementInt (Variables|Default|Getplayernum))
        (:%20%20
          (Variables|Default|Setplayernum _result)))))
  (bind _returnvalue (Class|GameModeBase|GetNumPlayers))
  (if (== (Variables|Default|Getplayernum) _returnvalue)
    (Default|Startvisivle _roommaster)
    (else
      (Default|Starthidden _roommaster))))

(event Custom|se1
  (CallFunction|Setsungmul))

(event Custom|setsungmul
  (bind _output_get (Variables|Default|Setcurrentsungmul (Math|Random|RandomInteger 3) :!label _label))
  (if (Utilities|Array|ContainsItem (Variables|Default|Getsungmularr) _output_get)
    (Utilities|FlowControl|Delay (Utilities|Time|GetWorldDeltaSeconds))
    (goto _label)
    (else
      (Utilities|Array|Add (Variables|Default|Getsungmularr) (Variables|Default|Getcurrentsungmul))
      (bind _output_get_2 (Variables|Default|Settemptrans (Utilities|Array|Get(acopy) (Variables|Default|Getspawntarget) (Math|Random|RandomInteger 6))))
      (Game|SpawnActorfromClass "/Game/sinyoung/new/sungmulactor.sungmulactor_C" _output_get_2 "AlwaysSpawn" 0 _output_get 0)
      (CallFunction|SetPar 0 (.Location (Math|Transform|BreakTransform _output_get_2)) (Variables|Default|Getcurrentsungmul)))))

(event Custom|se2
  (CallFunction|Setsungmul))

(event Custom|se3
  (CallFunction|Setsungmul))

(event Custom|set%20par
  (params (actiontype :type Integer) (transform :type Vector) (roottype :type Integer))
  (for _array_element (Variables|Default|GetAlivePCs)
    (Default|Spawnsungmul _array_element actiontype transform roottype)))

(event EventTick
  (params (DeltaSeconds :type Float%20%28single-precision%29)))

(event EventBeginPlay
  (bind _returnvalue (Utilities|Time|SetTimerbyEvent (delegate Custom|MainTimer) 1.0 true))
  (Variables|Default|SetMainTimerHandle _returnvalue))

(event EventPostLogin
  (params (NewPlayer :type Player%20Controller%20Object%20Reference))
  (bind _asbp_battle_pc (Utilities|Casting|CastToBP_BattlePC NewPlayer))
  (Utilities|Array|Add (Variables|Default|GetAlivePCs) _asbp_battle_pc))

(event EventOnLogout
  (params (ExitingController :type Controller%20Object%20Reference))
  (bind _asbp_battle_pc (Utilities|Casting|CastToBP_BattlePC ExitingController))
  (Utilities|Array|RemoveItem (Variables|Default|GetAlivePCs) _asbp_battle_pc))

(fn ConstructionScript)

(fn SaytoAll
  (params (Message :type String))
  (for _array_element (Variables|Default|GetAlivePCs)
    (Variables|/Game/Battle/BP_BattlePC.BP_BattlePC_C|SetNotificationFromServer _array_element Message)))